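; BP_Hazard is an area hazard that applies external heat to mechs standing inside it.
; On begin overlap it sets the CHR_Mech's ExternalHeat to HazardHeat, and on end overlap it resets that value to zero, with no handling for overlapping hazards.
; The construction script fits the Plane's height and horizontal scale to the Box's unscaled extent, so the visual matches the trigger volume.
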(event Collision|EventActorBeginOverlap
  (params (OtherActor :type Actor%20Object%20Reference))
  (bind _aschr_mech (Utilities|Casting|CastToCHR_Mech OtherActor))
  (Variables|/Game/Blueprints/PlayerCharacter/CHR_Mech.CHR_Mech_C|SetExternalHeat _aschr_mech (Variables|Default|GetHazardHeat)))

(event Collision|EventActorEndOverlap
  (params (OtherActor :type Actor%20Object%20Reference))
  (bind _aschr_mech (Utilities|Casting|CastToCHR_Mech OtherActor))
  (Variables|/Game/Blueprints/PlayerCharacter/CHR_Mech.CHR_Mech_C|SetExternalHeat _aschr_mech 0.0))

(fn ConstructionScript
  (bind _box (Variables|Default|GetBox))
  (bind _returnvalue (Components|Box|GetUnscaledBoxExtent _box))
  (bind (_x _y) (Class|KismetMathLibrary|BreakVector3f _returnvalue))
  (Transformation|SetRelativeLocation (Variables|Default|GetPlane) (Math|Vector|MakeVector 0.0 0.0 (.Z (Class|KismetMathLibrary|BreakVector3f (Components|Box|GetUnscaledBoxExtent (Variables|Default|GetBox))))) false false)
  (Transformation|SetRelativeScale3D (Variables|Default|GetPlane) (Math|Vector|MakeVector (* (/ _x 1e+02) 2.0) (* (/ _y 1e+02) 2.0) 1.0)))