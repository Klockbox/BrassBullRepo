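; BP_Interactor_Child is an interactor placed as a child actor on CHR_Mech that links to the turret in one of the mech's slots.
; On BeginPlay it casts its parent to CHR_Mech, picks the right or left turret slot component from AttachedToSlot, and caches that slot's PWN_Turret.
; Its interaction event calls the parent handler, then only prints the slot component and turret names as debug output.
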(event EventInteractionEvent
  (|CallParentFunction)
  (Development|PrintString (Utilities|GetObjectName (Variables|Default|GetChildActorComponentReference)))
  (Development|PrintString (Utilities|GetObjectName (Variables|Default|GetAttachedTurret))))

(event EventBeginPlay
  (bind _aschr_mech (Utilities|Casting|CastToCHR_Mech (Actor|GetParentActor)))
  (bind _output_get (Variables|Default|SetChildActorComponentReference (Utilities|Select :Index (Variables|Default|GetAttachedToSlot) :NewEnumerator0 (Variables|/Game/Blueprints/CHR_Mech.CHR_Mech_C|GetTurretSlot_Right _aschr_mech) :NewEnumerator1 (Variables|/Game/Blueprints/CHR_Mech.CHR_Mech_C|GetTurretSlot_Left _aschr_mech))))
  (bind _aspwn_turret (Utilities|Casting|CastToPWN_Turret (Variables|/Script/Engine.ChildActorComponent|GetChildActor _output_get))
    (:then
      (Variables|Default|SetAttachedTurret _aspwn_turret))
    (:CastFailed
      (Development|PrintString "Turret attachment did not work"))))

(fn ConstructionScript
  (|CallParentFunction))