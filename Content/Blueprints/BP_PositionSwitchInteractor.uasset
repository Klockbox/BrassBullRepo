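; Position switch interactor, a child actor in a mech or turret that moves Johanna between the cockpit and turret slots.
; On BeginPlay, ReferencingSlot implies the host type, and it caches the destination JohannaSlot through parent and child actor casts.
; In the mech, interaction releases control and sends Johanna immediately.
; In a turret, it starts rotation to base position if operating normally, leaving the send to OnTransitionRequirementMet, reachable through the turret's stored reference.
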(event Custom|On%20TransitionRequirementMet
  ;[1 1 1] Kick off "animation"
  (Default|SendJohannatoSlot (Variables|Default|GetJohanna) (Variables|Default|GetAttachedJohannaSlot)))

(event EventBaseInteractionEvent
  (|CallParentFunction)
  ;[1 1 1] Disable control of part (imagine Johanna moving hands away from the control.)
  (switch Utilities|FlowControl|Switch|SwitchonE_ReferencedChildActorSlot (Variables|PositionSwitchOptions|GetReferencing%20Slot) ; We can infer: \nWhen its refernecing turrets the part is placed in a mech. \nWhen its referencing the cockpit its in a turret.
    (:NewEnumerator0
      (Default|SetControlled (Variables|Default|GetParentMech) false :!label _label)
      ;[1 1 1] currently no plans on delaying
      (CallFunction|OnTransitionRequirementMet))
    (:NewEnumerator1
      (goto _label))
    (:NewEnumerator2
      (switch Utilities|FlowControl|Switch|SwitchonE_TurretStates (Variables|/Game/Blueprints/PWN_Turret.PWN_Turret_C|GetCurrentState (Variables|Default|GetParentTurret))
        (:NewEnumerator0
          ;[1 1 1] Turn turret to base Pos
          (Default|SetTurretState (Variables|Default|GetParentTurret) "NewEnumerator1"))))))

(event EventBeginPlay
  (bind _returnvalue (Actor|GetParentActor))
  (Utilities|FlowControl|Sequence
    (:then_0
      ;[1 1 1] make sure there is a parent actor
      (Utilities|IsValid _returnvalue
        (:Is%20Not%20Valid
          (Development|PrintString "Connector without parent found. Destroy.")
          (Actor|DestroyActor))))
    (:then_1
      (switch Utilities|FlowControl|Switch|SwitchonE_ReferencedChildActorSlot (Variables|PositionSwitchOptions|GetReferencing%20Slot) ; We can infer: \nWhen its refernecing turrets the part is placed in a mech. \nWhen its referencing the cockpit its in a turret.
        (:NewEnumerator0
          ;[1 1 1] Find and safe parent
          (bind _aschr_mech (Utilities|Casting|CastToCHR_Mech _returnvalue :!label _label)
            (:then
              (bind _output_get (Variables|Default|SetParentMech _aschr_mech))
              ;[1 1 1] Get the Johanna slot in the wished turret
              (bind _aspwn_turret (Utilities|Casting|CastToPWN_Turret (Variables|/Script/Engine.ChildActorComponent|GetChildActor (Utilities|Select :Index (Variables|PositionSwitchOptions|GetReferencing%20Slot) :NewEnumerator0 (Variables|/Game/Blueprints/CHR_Mech.CHR_Mech_C|GetTurretSlot_Right _output_get) :NewEnumerator1 (Variables|/Game/Blueprints/CHR_Mech.CHR_Mech_C|GetTurretSlot_Left _output_get) :NewEnumerator2 0)))
                (:then
                  (bind _asbp_johanna_slot (Utilities|Casting|CastToBP_JohannaSlot (Variables|/Script/Engine.ChildActorComponent|GetChildActor (Variables|/Game/Blueprints/PWN_Turret.PWN_Turret_C|GetBP_JohannaSlot _aspwn_turret)))
                    (:then
                      (Variables|Default|SetAttachedJohannaSlot _asbp_johanna_slot))
                    (:CastFailed
                      (Development|PrintString "Mech interactor can't Johanna slot in Turret"))))
                (:CastFailed
                  (Development|PrintString "Mech interactor can't find turret child"))))
            (:CastFailed
              (Development|PrintString "Interactor can't find mech parent"))))
        (:NewEnumerator1
          (goto _label))
        (:NewEnumerator2
          (bind _aspwn_turret_2 (Utilities|Casting|CastToPWN_Turret _returnvalue)
            (:then
              (bind _output_get_2 (Variables|Default|SetParentTurret _aspwn_turret_2))
              ;[1 1 1] Set reference in turret parent
              (Variables|/Game/Blueprints/PWN_Turret.PWN_Turret_C|SetPosSwitchInteractor _output_get_2 self)
              ;[1 1 1] Get the Johanna slot in the mech
              (bind _aschr_mech_2 (Utilities|Casting|CastToCHR_Mech (Actor|GetParentActor _output_get_2))
                (:then
                  (bind _asbp_johanna_slot_2 (Utilities|Casting|CastToBP_JohannaSlot (Variables|/Script/Engine.ChildActorComponent|GetChildActor (Variables|/Game/Blueprints/CHR_Mech.CHR_Mech_C|GetBP_JohannaSlot _aschr_mech_2)))
                    (:then
                      (Variables|Default|SetAttachedJohannaSlot _asbp_johanna_slot_2))
                    (:CastFailed
                      (Development|PrintString "Turret interactor can't Johanna slot in Mech"))))
                (:CastFailed
                  (Development|PrintString "Turret interactor can't find mech parent"))))
            (:CastFailed
              (Development|PrintString "Interactor can't find turret parent"))))))))

(fn ConstructionScript
  (|CallParentFunction))