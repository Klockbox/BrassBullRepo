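; CR_Mech is a mech Blueprint with a CharacterMovement component that tracks its own horizontal speed.
; On BeginPlay it finds the BB_PlayerController with GetActorOfClass, caches it as CharacterController and prints whether it was found.
; Each Tick it stores the XY length of the movement component's velocity in HorizontalVelocity.
; The cached controller is not used further in these graphs.
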(event EventBeginPlay
  (bind _returnvalue (Actor|GetActorOfClass "/Game/Blueprints/BB_PlayerController.BB_PlayerController_C"))
  (Utilities|IsValid _returnvalue
    (:Is%20Valid
      (Development|PrintString "CharacterController found")
      (Variables|Default|SetCharacterController _returnvalue))
    (:Is%20Not%20Valid
      (Development|PrintString "CharacterController not found"))))

(event EventTick
  (params (DeltaSeconds :type Float%20%28single-precision%29))
  (Utilities|FlowControl|Sequence
    (:then_0
      (CallFunction|GetHorizontalVelocity))))

(fn ConstructionScript)

(fn GetHorizontalVelocity
  (Variables|Default|SetHorizontalVelocity (Math|Vector|VectorLengthXY (Variables|/Script/Engine.MovementComponent|GetVelocity (Variables|Character|GetCharacterMovement)))))