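; Hit point component that tracks an actor's current HP, starting at either max or a set value, and marks it dead at zero.
; ChangeHP adds or sets HP, then fires death, damage or health-gained events, with no clamp at MaxHP.
; Helper checks compare HP before and after, intended as percentages, to fire one event for crossing the 25, 50 or 75 thresholds in either direction.
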(event EventBeginPlay
  (switch Utilities|FlowControl|Switch|SwitchonE_HealthStartOptions (Variables|HealthPoints|GetStart%20with)
    (:NewEnumerator0
      (Variables|HealthPoints|SetCurrentHP (Variables|HealthPoints|GetMaxHP)))
    (:NewEnumerator1
      (Variables|HealthPoints|SetCurrentHP (Variables|HealthPoints|GetStartHP)))))

(event EventTick
  (params (DeltaSeconds :type Float%20%28single-precision%29)))

(fn ChangeHP
  (params (Change%20mode :type E_HPChangeType%20Enum :default "NewEnumerator1") (Value :type Integer))
  (if (Variables|Default|GetIsDead)
    (return true)
    (else
      (LocalVariables|SetHP%20before (Variables|HealthPoints|GetCurrentHP))
      (LocalVariables|SetHP%25%20before (|CalcHP%before))
      (switch Utilities|FlowControl|Switch|SwitchonE_HPChangeType Change%20mode
        (:NewEnumerator1
          (Variables|HealthPoints|SetCurrentHP (+ Value (Variables|HealthPoints|GetCurrentHP))))
        (:NewEnumerator0
          (Variables|HealthPoints|SetCurrentHP Value)))
      (LocalVariables|SetHP%25%20now (|CalcHP%now))
      (if (< (Variables|HealthPoints|GetCurrentHP) (LocalVariables|GetHP%20before))
        ;[1 0 0.053] HP loss
        (if (<= (Variables|HealthPoints|GetCurrentHP) 0)
          ;;[0 0 0] Actor dies
          (Variables|HealthPoints|SetCurrentHP 0)
          (Default|CallOnDeath)
          (Variables|Default|SetIsDead true)
          (else
            (Default|CallOnDamageTaken)
            (bind _returnvalue (CallFunction|DidHPFallBelowThreshold? 25.0 (LocalVariables|GetHP%25%20before) (LocalVariables|GetHP%25%20now)))
            (if _returnvalue
              (Default|CallHPFellBelow25%)
              (else
                (bind _returnvalue_2 (CallFunction|DidHPFallBelowThreshold? 5e+01 (LocalVariables|GetHP%25%20before) (LocalVariables|GetHP%25%20now)))
                (if _returnvalue_2
                  (Default|CallHPFellBelow50%)
                  (else
                    (bind _returnvalue_3 (CallFunction|DidHPFallBelowThreshold? 75.0 (LocalVariables|GetHP%25%20before) (LocalVariables|GetHP%25%20now)))
                    (if _returnvalue_3
                      (Default|CallHPFellBelow75%))))))))
        (else
          ;[0.1667 1 0.2621] HP gain
          (Default|CallOnHealthGained)
          (bind _returnvalue_4 (CallFunction|DidHPRiseAboveThreshold? 75.0 (LocalVariables|GetHP%25%20before) (LocalVariables|GetHP%25%20now)))
          (if _returnvalue_4
            (Default|CallHPRoseAbove75%)
            (else
              (bind _returnvalue_5 (CallFunction|DidHPRiseAboveThreshold? 5e+01 (LocalVariables|GetHP%25%20before) (LocalVariables|GetHP%25%20now)))
              (if _returnvalue_5
                (Default|CallHPRoseAbove50%)
                (else
                  (bind _returnvalue_6 (CallFunction|DidHPRiseAboveThreshold? 25.0 (LocalVariables|GetHP%25%20before) (LocalVariables|GetHP%25%20now)))
                  (if _returnvalue_6
                    (Default|CallHPRoseAbove25%)))))))))))

(fn DidHPFallBelowThreshold?
  (params (Threshold :type Float%20%28double-precision%29) (HP%25%20before :type Float%20%28double-precision%29) (HP%25%20now :type Float%20%28double-precision%29))
  (return (and (>= HP%25%20before Threshold) (< HP%25%20now Threshold))))

(fn DidHPRiseAboveThreshold?
  (params (Threshold :type Float%20%28double-precision%29) (HP%25%20before :type Float%20%28double-precision%29) (HP%25%20now :type Float%20%28double-precision%29))
  (return (and (< HP%25%20before Threshold) (>= HP%25%20now Threshold))))