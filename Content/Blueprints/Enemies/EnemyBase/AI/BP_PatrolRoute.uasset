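; BP_PatrolRoute is a patrol route for enemy AI, built on a Route spline whose points are tracked by index.
; Its IncrementPatrolRoute event takes direction and patrol type but is empty.
; Unconnected ping-pong logic steps PatrolIndex along the spline points and flips PatrolDirection at either end.
; A note says patrol behavior will move to BaseEnemy, and the construction script is empty.
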(event Custom|IncrementPatrolRoute
  (params (AI%20Patrol%20Direction :type E_PatrolDirection%20Enum :default "NewEnumerator0") (AI%20Patrol%20Type :type E_PatrolPathType%20Enum :default "NewEnumerator0"))
  ;[1 1 0] PatrolBehavior will be moved to BaseEnemy
)

(fn ConstructionScript)