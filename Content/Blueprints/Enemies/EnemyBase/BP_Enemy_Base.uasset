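; Base enemy character, driven by AIC_Enemy_Base, with spline patrolling, speed tiers, health and a telegraphed laser attack.
; Fire locks a slightly randomized direction toward the blackboard target; Tick animates the Niagara aim beam until AimTime elapses with a blocking hit.
; Fire2 then re-traces, applies damage and signals completion.
; HitPointSystem reports damage to AI perception as caused by CHR_Mech and destroys the actor on death.
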(event OnDeath(HitPointSystem)
  (Actor|DestroyActor))

(event OnDamageTaken(HitPointSystem)
  (params (DamageTaken :type Integer) (Instigator :type Actor%20Object%20Reference) (HitLocation :type Vector :default "0, 0, 0"))
  (bind _returnvalue (Actor|GetActorOfClass "/Game/Blueprints/PlayerCharacter/CHR_Mech.CHR_Mech_C"))
  (Class|AISenseDamage|ReportDamageEvent self _returnvalue 0.0 "0, 0, 0" "0, 0, 0" "None"))

(event Custom|AimAtTarget
  ;[1 1 0] unused
  (Default|CallAimingDone true))

(event Custom|Fire
  (bind _returnvalue (Math|Random|RandomFloatinRange -1.0 1.0))
  (bind _charactercontroller (Variables|References|GetCharacterController))
  (Components|Activation|Activate (Variables|Default|GetNS_Laser) false)
  (bind _asactor (Utilities|Casting|CastToActor (AI|Components|Blackboard|GetValueasObject (AI|GetBlackboard _charactercontroller) (Variables|/Game/Blueprints/Enemies/EnemyBase/AI/AIC_Enemy_Base.AIC_Enemy_Base_C|GetAttackTarget%20Key%20Name _charactercontroller))))
  (Variables|Default|SetAimDirectionVector (Math|Vector|RotateVector (Math|Vector|Normalize (- (Transformation|GetActorLocation _asactor) (Transformation|GetWorldLocation (Variables|Default|GetPlaceholder%20BeamStart)))) (Math|Rotator|MakeRotator 0.0 _returnvalue _returnvalue)))
  (Variables|Default|SetLaserAiming true))

(event Custom|Fire2
  (bind _placeholder_beamstart (Variables|Default|GetPlaceholder%20BeamStart))
  (bind _returnvalue (Transformation|GetWorldLocation _placeholder_beamstart))
  (Components|Activation|Deactivate (Variables|Default|GetNS_Laser))
  (Variables|Default|SetLaserAiming false)
  (Variables|Default|SetTimer 0.0)
  (Niagara|SetNiagaraVariable(Float) (Variables|Default|GetNS_Laser) "AimBeamAgeNormalized" 0.0)
  (bind _outhit (Collision|LineTraceForObjects _returnvalue (+ _returnvalue (* (Variables|Default|GetAimDirectionVector) (Variables|Default|GetLaserMaxLenght))) (Variables|Default|GetObject%20Types) false 0 "None"))
  (Class|BPIDamageableEntity|ChangeEntityHP(Message) (.HitActor (Collision|BreakHitResult _outhit)) "NewEnumerator1" -10 (.ImpactPoint (Collision|BreakHitResult _outhit)) self)
  (bind _returnvalue_2 (Niagara|SpawnSystematLocation "/Game/Effects/ParticleEffects/NS_LaserFire.NS_LaserFire" "0, 0, 0"))
  (Niagara|SetNiagaraVariable(Vector3) _returnvalue_2 "StartPoint" _returnvalue)
  (Niagara|SetNiagaraVariable(Vector3) _returnvalue_2 "EndPoint" (.ImpactPoint (Collision|BreakHitResult _outhit)))
  (Default|CallFiringDone true))

(event EventPossessed
  (params (NewController :type Controller%20Object%20Reference))
  (bind _asaic_enemy_base (Utilities|Casting|CastToAIC_Enemy_Base NewController)
    (:then
      (Variables|References|SetCharacterController _asaic_enemy_base)
      (Variables|Default|SetLaserAiming false)
      (Variables|Default|SetTimer 0.0)
      (Niagara|SetNiagaraVariable(Float) (Variables|Default|GetNS_Laser) "AimBeamAgeNormalized" 0.0))
    (:CastFailed
      (Development|PrintString "Enemy Base is controlled by worng ai controller. delete.")
      (Actor|DestroyActor))))

(event EventTick
  (params (DeltaSeconds :type Float%20%28single-precision%29))
  (bind _placeholder_beamstart (Variables|Default|GetPlaceholder%20BeamStart))
  (bind _returnvalue (Transformation|GetWorldLocation _placeholder_beamstart))
  (if (Variables|Default|GetLaserAiming)
    (bind _output_get (Variables|Default|SetTimer (+ (Utilities|Time|GetWorldDeltaSeconds) (Variables|Default|GetTimer))))
    (Niagara|SetNiagaraVariable(Float) (Variables|Default|GetNS_Laser) "AimBeamAgeNormalized" (/ _output_get (Variables|Default|GetAimTime)))
    (bind _outhit (Collision|LineTraceForObjects _returnvalue (+ _returnvalue (* (Variables|Default|GetAimDirectionVector) (Variables|Default|GetLaserMaxLenght))) (Variables|Default|GetObject%20Types) false 0 "None"))
    (if (.bBlockingHit (Collision|BreakHitResult _outhit))
      (Niagara|SetNiagaraVariable(Vector3) (Variables|Default|GetNS_Laser) "BeamEnd" (.Location (Collision|BreakHitResult _outhit)))
      (if (>= (Variables|Default|GetTimer) (Variables|Default|GetAimTime))
        (CallFunction|Fire2)))))

(fn ConstructionScript)

(fn IncrementPatrolRoute
  (if (Variables|AI|GetJumpToOtherEndPoint)
    (if (<= (Variables|AI|GetPatrolRouteIndex) 0)
      ;[1 1 1] When entity is at 0 point, go to far end point next
      (Variables|AI|SetPatrolRouteIndex (- (Spline|GetNumberOfSplinePoints (Variables|/Game/Blueprints/Enemies/EnemyBase/AI/BP_PatrolRoute.BP_PatrolRoute_C|GetRoute (Variables|AI|GetPatrolRoute))) 1))
      (else
        ;[1 1 1] When entity is at far point go to 0 point
        (Variables|AI|SetPatrolRouteIndex 0)))
    (Variables|AI|SetJumpToOtherEndPoint false)
    (else
      (Variables|AI|SetPatrolRouteIndex (+ (Variables|AI|GetPatrolRouteIndex) (Utilities|Select :Index (Variables|AI|GetPatrolDirection) :NewEnumerator0 1 :NewEnumerator1 -1)))
      ;[1 1 1] Check for end point
      (if (Utilities|Select :Index (Variables|AI|GetPatrolDirection) :NewEnumerator0 (== (Variables|AI|GetPatrolRouteIndex) (- (Spline|GetNumberOfSplinePoints (Variables|/Game/Blueprints/Enemies/EnemyBase/AI/BP_PatrolRoute.BP_PatrolRoute_C|GetRoute (Variables|AI|GetPatrolRoute))) 1)) :NewEnumerator1 (<= (Variables|AI|GetPatrolRouteIndex) 0))
        (switch Utilities|FlowControl|Switch|SwitchonE_PatrolPathType (Variables|AI|GetPatrolType)
          (:NewEnumerator0
            ;[1 1 1] Flip direction
            (switch Utilities|FlowControl|Switch|SwitchonE_PatrolDirection (Variables|AI|GetPatrolDirection)
              (:NewEnumerator0
                (Variables|AI|SetPatrolDirection "NewEnumerator1"))
              (:NewEnumerator1
                (Variables|AI|SetPatrolDirection "NewEnumerator0"))))
          (:NewEnumerator1
            ;[1 1 1] Entity reached end point and needs to go to the other end point next
            (Variables|AI|SetJumpToOtherEndPoint true)))))))

(fn ChangeEntityHP
  (params (HP%20Change%20Mode :type E_HPChangeType%20Enum :default "NewEnumerator1") (Value :type Integer) (HitLocation :type Vector :default "0, 0, 0") (Instigator :type Actor%20Object%20Reference))
  (bind _isded (Default|ChangeHP (Variables|Default|GetHitPointSystem) HP%20Change%20Mode Value "0, 0, 0"))
  (return true _isded))

(fn GetCharacterMovementComponent
  (return (Variables|Character|GetCharacterMovement)))

(fn GetEntityPassiveTask
  (return (Variables|AI|GetDesiredPassiveTask)))

(fn GetGroundWorldPosition
  (bind _returnvalue (Transformation|GetActorLocation))
  (bind (_x _y _z) (Math|Vector|BreakVector _returnvalue))
  (return (Math|Vector|MakeVector _x _y (- _z (Components|Capsule|GetScaledCapsuleHalfHeight (Variables|Collision|GetCapsuleComponent))))))

(fn GetHealthComponent
  (return (Variables|Default|GetHitPointSystem)))

(fn GetPatrolPointWorldPosition
  (bind _output_get (Variables|AI|SetCurrentMoveTarget (Spline|GetLocationatSplinePoint (Variables|/Game/Blueprints/Enemies/EnemyBase/AI/BP_PatrolRoute.BP_PatrolRoute_C|GetRoute (Variables|AI|GetPatrolRoute)) (Variables|AI|GetPatrolRouteIndex) "World")))
  (return _output_get))

(fn GetPatrolRoute
  (return (Variables|AI|GetPatrolRoute)))

(fn IncrementPatrolPoint
  (if (Variables|AI|GetJumpToOtherEndPoint)
    (if (<= (Variables|AI|GetPatrolRouteIndex) 0)
      ;[1 1 1] When entity is at 0 point, go to far end point next
      (Variables|AI|SetPatrolRouteIndex (- (Spline|GetNumberOfSplinePoints (Variables|/Game/Blueprints/Enemies/EnemyBase/AI/BP_PatrolRoute.BP_PatrolRoute_C|GetRoute (Variables|AI|GetPatrolRoute))) 1))
      (else
        ;[1 1 1] When entity is at far point go to 0 point
        (Variables|AI|SetPatrolRouteIndex 0)))
    (Variables|AI|SetJumpToOtherEndPoint false)
    (else
      (Variables|AI|SetPatrolRouteIndex (+ (Variables|AI|GetPatrolRouteIndex) (Utilities|Select :Index (Variables|AI|GetPatrolDirection) :NewEnumerator0 1 :NewEnumerator1 -1)))
      ;[1 1 1] Check for end point
      (if (Utilities|Select :Index (Variables|AI|GetPatrolDirection) :NewEnumerator0 (== (Variables|AI|GetPatrolRouteIndex) (- (Spline|GetNumberOfSplinePoints (Variables|/Game/Blueprints/Enemies/EnemyBase/AI/BP_PatrolRoute.BP_PatrolRoute_C|GetRoute (Variables|AI|GetPatrolRoute))) 1)) :NewEnumerator1 (<= (Variables|AI|GetPatrolRouteIndex) 0))
        (switch Utilities|FlowControl|Switch|SwitchonE_PatrolPathType (Variables|AI|GetPatrolType)
          (:NewEnumerator0
            ;[1 1 1] Flip direction
            (switch Utilities|FlowControl|Switch|SwitchonE_PatrolDirection (Variables|AI|GetPatrolDirection)
              (:NewEnumerator0
                (Variables|AI|SetPatrolDirection "NewEnumerator1"))
              (:NewEnumerator1
                (Variables|AI|SetPatrolDirection "NewEnumerator0"))))
          (:NewEnumerator1
            ;[1 1 1] Entity reached end point and needs to go to the other end point next
            (Variables|AI|SetJumpToOtherEndPoint true))))))
  (return))

(fn SetMovementSpeed
  (params (MovementSpeed :type E_MovementSpeed%20Enum :default "NewEnumerator4"))
  (bind _output_get (Variables|/Script/Engine.CharacterMovementComponent|SetMaxWalkSpeed (Variables|Character|GetCharacterMovement) (Utilities|Select :Index MovementSpeed :NewEnumerator4 0.0 :NewEnumerator1 (Variables|AI|GetPatrol%20Speed) :NewEnumerator3 (Variables|AI|GetAgitated%20Speed) :NewEnumerator0 (Variables|AI|GetFull%20Speed))))
  (return _output_get))