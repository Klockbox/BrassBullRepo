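; Enemy laser gun that fires a telegraphed hitscan shot at a target location, then signals attack completion after a cooldown.
; Attack locks the aim direction and starts a Niagara aim beam, which Tick ages over the charge time while re-tracing its end point from the muzzle.
; When charged, Fire line-traces along that direction, sends HP damage to any hit actor and spawns a beam effect to the impact point.
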(event Custom|Charge
  (Development|PrintString "Enemy Laser Charging" true false "(R=1.000000,G=0.455003,B=0.415181,A=1.000000)" 0.0)
  (Utilities|FlowControl|Sequence
    (:then_0
      ;[1 1 1] Count up timer
      (Variables|Default|SetTimer (+ (Utilities|Time|GetWorldDeltaSeconds) (Variables|Default|GetTimer))))
    (:then_1
      ;[1 1 1] Set Niagara System Age
      (Niagara|SetNiagaraVariable(Float) (Variables|Default|GetNS_Laser) "AimBeamAgeNormalized" (/ (Variables|Default|GetTimer) (Variables|Default|GetChargeTime))))
    (:then_2
      ;[1 1 1] Set Laser End
      (CallFunction|SetAimLaserEndPoint))
    (:then_3
      ;[1 1 1] Done charging?
      (if (>= (Variables|Default|GetTimer) (Variables|Default|GetChargeTime))
        ;[1 1 1] Done charging!
        (Variables|Default|SetCharging false)
        (Variables|Default|SetTimer 0.0)
        (Niagara|SetNiagaraVariable(Float) (Variables|Default|GetNS_Laser) "AimBeamAgeNormalized" 0.0)
        (Components|Activation|Deactivate (Variables|Default|GetNS_Laser))
        (CallFunction|Fire)))))

(event Custom|Attack
  (params (TargetLocation :type Vector))
  (CallFunction|Aim TargetLocation))

(event Custom|Aim
  (params (Target :type Vector))
  ;[1 1 1] Set Aim + Random Offset
  (Variables|Default|SetAimDirectionVector (|GetDirectionVectorToTarget Target))
  (CallFunction|SetAimLaserEndPoint)
  (Components|Activation|Activate (Variables|Default|GetNS_Laser) false)
  (Variables|Default|SetCharging true)
  (Development|PrintString "Aiming Done"))

(event Custom|Fire
  (Development|PrintString "Enemy Laser FIRE!" true false "(R=1.000000,G=0.455003,B=0.415181,A=1.000000)")
  ;[1 1 1] Hitscan
  (bind _output_get (Variables|Default|SetImpact%20Point (+ (Variables|Default|GetMuzzleLocation) (* (Variables|Default|GetAimDirectionVector) (Variables|Default|GetLaserMaxLenght))))) ; Needs to be set here, if there\nis no other laser contact.\nWill be overwritten by impact point\n     if trace returns hit.
  (bind (_outhit _returnvalue) (Collision|LineTraceForObjects (Variables|Default|GetMuzzleLocation) _output_get (Variables|Default|GetObject%20Types) false 0 "None"))
  (Utilities|FlowControl|Sequence
    (:then_0
      ;[1 1 1] Deal Damage
      (if _returnvalue
        (Variables|Default|SetImpact%20Point (.ImpactPoint (Collision|BreakHitResult _outhit)))
        (Class|BPIDamageableEntity|ChangeEntityHP(Message) (.HitActor (Collision|BreakHitResult _outhit)) "NewEnumerator1" -10 "NewEnumerator1" (Variables|Default|GetImpact%20Point) self)))
    (:then_1
      ;[1 1 1] Spawn Laser Niagara Effect
      (bind _returnvalue_2 (Niagara|SpawnSystematLocation "/Game/Effects/ParticleEffects/NS_LaserFire.NS_LaserFire" (Variables|Default|GetMuzzleLocation)))
      (Niagara|SetNiagaraVariable(Vector3) _returnvalue_2 "StartPoint" (Variables|Default|GetMuzzleLocation))
      (Niagara|SetNiagaraVariable(Vector3) _returnvalue_2 "EndPoint" (Variables|Default|GetImpact%20Point)))
    (:then_2
      ;[1 1 1] Call that the attack is done
      (Utilities|FlowControl|Delay (Variables|Default|GetAfterAttackCooldown))
      (Default|CallAttackFinished))))

(event EventTick
  (params (DeltaSeconds :type Float%20%28single-precision%29))
  (Utilities|FlowControl|Sequence
    (:then_0
      (Variables|Default|SetMuzzleLocation (Transformation|GetWorldLocation (Variables|Default|GetMuzzle))))
    (:then_1
      (if (Variables|Default|GetCharging)
        (CallFunction|Charge)))))

(fn ConstructionScript)

(fn SetAimLaserEndPoint
  (bind _aimdirectionvector (Variables|Default|GetAimDirectionVector))
  (bind _lasermaxlenght (Variables|Default|GetLaserMaxLenght))
  (bind _muzzlelocation (Variables|Default|GetMuzzleLocation))
  (bind _returnvalue (* _aimdirectionvector _lasermaxlenght))
  (bind _returnvalue_2 (+ _muzzlelocation _returnvalue))
  (bind _outhit (Collision|LineTraceForObjects _muzzlelocation _returnvalue_2 (Variables|Default|GetObject%20Types) false 0 "None"))
  (if (.bBlockingHit (Collision|BreakHitResult _outhit))
    (Niagara|SetNiagaraVariable(Vector3) (Variables|Default|GetNS_Laser) "BeamEnd" (.Location (Collision|BreakHitResult _outhit)))
    (else
      (Niagara|SetNiagaraVariable(Vector3) (Variables|Default|GetNS_Laser) "BeamEnd" _returnvalue_2))))