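; Player controller Blueprint that sets up Enhanced Input and holds placeholder handlers for interact and view-unlock actions.
; On BeginPlay it casts player controller 0 to its own class and adds the Default mapping context, printing whether this succeeded.
; The interact handler fires on Started and the view-unlock handler on Started and Completed; all only print debug messages.
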(event Input|EnhancedActionEvents|EnhancedInputActionIA_Interact
  (params (ActionValue :type Boolean) (ElapsedSeconds :type Float%20%28double-precision%29) (TriggeredSeconds :type Float%20%28double-precision%29) (InputAction :type Input%20Action%20Object%20Reference :default "/Game/Input/IA_Interact.IA_Interact"))
  (:Started
    (Development|PrintString "IA_Interact")))

(event Input|EnhancedActionEvents|EnhancedInputActionIA_UnlockView
  (params (ActionValue :type Boolean) (ElapsedSeconds :type Float%20%28double-precision%29) (TriggeredSeconds :type Float%20%28double-precision%29) (InputAction :type Input%20Action%20Object%20Reference :default "/Game/Input/IA_UnlockView.IA_UnlockView"))
  (:Started
    (Development|PrintString "IA_UnlockView started"))
  (:Completed
    (Development|PrintString "IA_UnlockView ended")))

(event EventBeginPlay
  (bind _aspc_controller (Utilities|Casting|CastToPC_Controller (Game|GetPlayerController 0))
    (:then
      (Input|AddMappingContext (PlayerController|LocalPlayerSubsystems|GetEnhancedInputLocalPlayerSubsystem _aspc_controller) "/Game/Input/Default.Default" 0 "(bIgnoreAllPressedKeysUntilRelease=True,bForceImmediately=False)")
      (Development|PrintString "Enhanced Input initialized"))
    (:CastFailed
      (Development|PrintString "PlayerIndex0 has wrong PlayerController"))))

(event EventTick
  (params (DeltaSeconds :type Float%20%28single-precision%29)))

(fn ConstructionScript)