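; Johanna pawn with an optional free-look camera driven by the player controller found at BeginPlay.
; While the controller's camera is unlocked, directional input rotates the camera within clamped yaw and pitch limits.
; Otherwise, a delta-time-scaled lerp eases it back to zero relative rotation.
; Tick also checks the current occupation and moves the pawn to world origin while it is In Transition.
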(event EventBeginPlay
  (bind _returnvalue (Actor|GetActorOfClass "/Game/Blueprints/PC_PlayerController.PC_PlayerController_C"))
  (Utilities|IsValid _returnvalue
    (:Is%20Valid
      (Development|PrintString "CharacterController found")
      (Variables|Default|SetCharacterController _returnvalue))
    (:Is%20Not%20Valid
      (Development|PrintString "CharacterController not found"))))

(event EventTick
  (params (DeltaSeconds :type Float%20%28single-precision%29))
  (Variables|Default|SetDeltaTime DeltaSeconds)
  (Utilities|FlowControl|Sequence
    (:then_0
      ;[1 1 1] Free Camera View
      ;;[1 1 1] additional check if I ever want to disable this feature
      (if (Variables|Default|GetAllowFreeCamera)
        (if (Variables|/Game/Blueprints/PC_PlayerController.PC_PlayerController_C|GetCameraUnlocked (Variables|Default|GetCharacterController))
          (CallFunction|RotateCamera)
          (else
            (CallFunction|RotateCameraBack)))))
    (:then_1
      (switch Utilities|FlowControl|Switch|SwitchonJohannaStates (Variables|Default|GetCurrentOccupation)
        (:NewEnumerator1
          (Transformation|SetActorLocation "0, 0, 0" false false))))))

(fn ConstructionScript)

(fn RotateCamera
  (bind _charactercontroller (Variables|Default|GetCharacterController))
  (bind _camera (Variables|Default|GetCamera))
  (bind _maxviewangles (Variables|Default|GetMaxViewAngles))
  (bind (_x _y) (Math|Vector2D|BreakVector2D _maxviewangles))
  (bind _directionalinput (Variables|/Game/Blueprints/PC_PlayerController.PC_PlayerController_C|GetDirectionalInput _charactercontroller))
  (bind _relativerotation (Variables|/Script/Engine.SceneComponent|GetRelativeRotation _camera))
  (bind (_x_2 _y_2) (Math|Vector2D|BreakVector2D _directionalinput))
  (bind (_roll _pitch _yaw) (Math|Rotator|BreakRotator _relativerotation))
  (Transformation|AddRelativeRotation (Variables|Default|GetCamera) (Math|Rotator|MakeRotator 0.0 _y_2 _x_2) false false)
  (Transformation|SetRelativeRotation (Variables|Default|GetCamera) (Math|Rotator|MakeRotator 0.0 (Math|Float|Clamp(Float) _pitch (* _y -1.0) _y) (Math|Float|Clamp(Float) _yaw (* _x -1.0) _x)) false false))

(fn RotateCameraBack
  (if (Utilities|Operators|NotEqual(!=) :A (Variables|/Script/Engine.SceneComponent|GetRelativeRotation (Variables|Default|GetCamera)) :ErrorTolerance 0.001)
    (Transformation|SetRelativeRotation (Variables|Default|GetCamera) (Math|Rotator|Lerp(Rotator) (Variables|/Script/Engine.SceneComponent|GetRelativeRotation (Variables|Default|GetCamera)) "0, 0, 0" (* (Variables|Default|GetDeltaTime) (Variables|Default|GetCamReturnSpeed))) false false)))