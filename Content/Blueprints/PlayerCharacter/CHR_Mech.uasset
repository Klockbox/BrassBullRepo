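; Player-piloted walking mech character, steered from a cockpit through a virtual stick.
; Tick turns clamped, accumulated stick input into turning and eased engine power, which sets walk speed and drives forward movement.
; A placeholder timeline sways the cockpit and triggers step shakes, while frame-compared wall hits separate crash from scraping shakes.
; Damage events add shake and knockback, death spawns an effect and destroys the actor, and debug prints remain throughout.
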(event Custom|OnHitWall
  (bind _charactermovement (Variables|Character|GetCharacterMovement))
  (bind _wallcollisionseverety (Variables|MechInfos|GetWallCollisionSeverety))
  (bind _mechmaxspeed (Variables|MechOptions|GetMechMaxSpeed))
  (bind _maxwalkspeed (Variables|/Script/Engine.CharacterMovementComponent|GetMaxWalkSpeed _charactermovement))
  (bind _returnvalue (/ _maxwalkspeed _mechmaxspeed))
  (bind _returnvalue_2 (* _wallcollisionseverety _returnvalue))
  (Development|PrintString (Utilities|String|Append (Utilities|String|MakeLiteralString "Collision severity: ") (Utilities|String|ToString(Float) _returnvalue_2)))
  (CameraShakes|StartCameraShake (Variables|/Script/Engine.PlayerController|GetPlayerCameraManager (Variables|References|GetPlayerController)) "/Game/Effects/CS_WallCrash.CS_WallCrash_C" _returnvalue_2 "CameraLocal" "0, 0, 0"))

(event Custom|OnStep
  (CameraShakes|StartCameraShake (Variables|/Script/Engine.PlayerController|GetPlayerCameraManager (Variables|References|GetPlayerController)) "/Game/Effects/CS_Step.CS_Step_C" (/ (Variables|/Script/Engine.CharacterMovementComponent|GetMaxWalkSpeed (Variables|Character|GetCharacterMovement)) (Variables|MechOptions|GetMechMaxSpeed)) "CameraLocal" "0, 0, 0"))

(event Custom|OnMechStart
  (CameraShakes|StartCameraShake (Variables|/Script/Engine.PlayerController|GetPlayerCameraManager (Variables|References|GetPlayerController)) "/Game/Effects/CS_MotorStart.CS_MotorStart_C" 1.0 "CameraLocal" "0, 0, 0"))

(event EventBeginPlay
  (Utilities|FlowControl|Sequence
    (:then_0
      ;[1 1 0] Starting placeholder Timeline Animation for Cockpit swaying
      (Variables|MechInfos|SetDebugAnimBasePos (Transformation|GetRelativeTransform (Variables|Default|GetCockpitBase))))
    (:then_1
      (bind (_direction _xbobbing _ybobbing _zbobbing _pitchswaying _rollswaying) (Timeline|DebugMechMovement Play)
        (:Update
          (Transformation|SetRelativeTransform (Variables|Default|GetCockpitBase) (Math|Transform|MakeTransform (Math|Vector|MakeVector (+ (* _xbobbing 0.2) (.X (Class|KismetMathLibrary|BreakVector3f (.Location (Math|Transform|BreakTransform (Variables|MechInfos|GetDebugAnimBasePos)))))) (+ (* _ybobbing 3e+01) (.Y (Class|KismetMathLibrary|BreakVector3f (.Location (Math|Transform|BreakTransform (Variables|MechInfos|GetDebugAnimBasePos)))))) (+ (* _zbobbing 4e+01) (.Z (Class|KismetMathLibrary|BreakVector3f (.Location (Math|Transform|BreakTransform (Variables|MechInfos|GetDebugAnimBasePos))))))) (Math|Rotator|MakeRotator (+ (* _rollswaying 0.5) (.Roll (Math|Rotator|BreakRotator (.Rotation (Math|Transform|BreakTransform (Variables|MechInfos|GetDebugAnimBasePos)))))) (+ (* _pitchswaying 1.0) (.Pitch (Math|Rotator|BreakRotator (.Rotation (Math|Transform|BreakTransform (Variables|MechInfos|GetDebugAnimBasePos)))))) (.Yaw (Math|Rotator|BreakRotator (.Rotation (Math|Transform|BreakTransform (Variables|MechInfos|GetDebugAnimBasePos))))))) false false)
          (Components|Timeline|SetPlayRate (Variables|Default|GetDebugMechMovement) (/ (/ (Variables|MechInfos|GetHorizontalVelocity) (Variables|/Script/Engine.CharacterMovementComponent|GetMaxWalkSpeed (Variables|Character|GetCharacterMovement))) 1.7)))
        (:EventTrack
          (CallFunction|OnStep))))
    (:then_2
      ;[1 1 0.003206] Saving placeholder steer stick base rot
      (Variables|MechInfos|SetPlacholderSteerStickRot (Variables|/Script/Engine.SceneComponent|GetRelativeRotation (Variables|Default|GetSteerStick))))
    (:then_3
      ;[1 1 0] Disable ticks until player controller enables it
      (Actor|Tick|SetActorTickEnabled false) ; Debug here: Simulating requires to turn of ticking. WIll be enabled when player controller sets reference
    )))

(event EventTick
  (params (DeltaSeconds :type Float%20%28single-precision%29))
  (bind _returnvalue (|CalculatePower-Speeddecrepancy))
  (Variables|Default|SetDeltaTime DeltaSeconds)
  (Utilities|FlowControl|Sequence
    (:then_0
      (CallFunction|Steering))
    (:then_1
      ;[1 1 0] Setting playbackspeed of placeholder animations
      (Components|Timeline|SetPlayRate (Variables|Default|GetDebugMechMovement) (/ (- (Variables|MechInfos|GetCurrentMechEnginePower) (/ (Variables|MechInfos|GetWallCollisionSeverety) 2.0)) 1.7)))
    (:then_2
      (Development|PrintString (Utilities|String|Append (Utilities|String|MakeLiteralString "Power-Speed Decrepancy: ") (Utilities|String|ToString(Float) _returnvalue)) true false "(R=0.000000,G=0.660000,B=1.000000,A=1.000000)" 0.0)
      (Development|PrintString (Utilities|String|Append (Utilities|String|MakeLiteralString "Heat built up: ") (Utilities|String|ToString(Float) (* (Math|Float|Clamp(Float) (- _returnvalue 0.5)) 2.0))) true false "(R=0.000000,G=0.660000,B=1.000000,A=1.000000)" 0.0))
    (:then_3
      ;[1 1 1] Compare the Hit Event to the last frame to register when a wall collission started and when it ended.
      (if (Variables|Default|GetWallHitThisFrame)
        (if (not (Variables|Default|GetWallHitLastFrame))
          (Variables|Default|SetWallHitLastFrame true)
          (CallFunction|OnHitWall))
        (elif (Variables|Default|GetWallHitLastFrame)
          (Variables|Default|SetWallHitLastFrame false))))
    (:then_4
      (Variables|MechInfos|SetWallCollisionSeverety 0.0)
      (Variables|Default|SetWallHitThisFrame false))))

(event Collision|EventHit
  (params (MyComp :type Primitive%20Component%20Object%20Reference) (Other :type Actor%20Object%20Reference) (OtherComp :type Primitive%20Component%20Object%20Reference) (bSelfMoved :type Boolean) (HitLocation :type Vector :default "0, 0, 0") (HitNormal :type Vector :default "0, 0, 0") (NormalImpulse :type Vector :default "0, 0, 0") (Hit :type Hit%20Result%20Structure%20%28by%20ref%29))
  (bind _returnvalue (Transformation|GetActorForwardVector))
  (bind _returnvalue_2 (* _returnvalue -1.0))
  (bind _returnvalue_3 (Class|KismetMathLibrary|VectorCosineAngle2D HitNormal _returnvalue_2))
  ;[1 1 1] Wall Scraping
  ;;[1 1 1] I want to check the collisions for geometry thats inhibiting movement to start effects and affect animations.
  ;; Therefore, I weed out collisions with the ground (not inhibting) and non static collisions.
  (if (and (== (Utilities|GetClass Other) "/Script/Engine.StaticMeshActor") (< (.Z (Class|KismetMathLibrary|BreakVector3f HitNormal)) 0.5))
    (Development|PrintString (Utilities|GetDisplayName Other) true false "(R=0.000000,G=0.660000,B=1.000000,A=1.000000)" 0.0)
    (Development|PrintString "+++HitEvent+++" false)
    (Variables|Default|SetWallHitThisFrame true)
    (Development|PrintString (Utilities|String|ToString(Float) _returnvalue_3) false)
    (bind _output_get (Variables|MechInfos|SetWallCollisionSeverety _returnvalue_3))
    (CameraShakes|StartCameraShake (Variables|/Script/Engine.PlayerController|GetPlayerCameraManager (Variables|References|GetPlayerController)) "/Game/Effects/CS_WallScraping.CS_WallScraping_C" (/ (+ (- 1.0 _output_get) (/ (Variables|/Script/Engine.CharacterMovementComponent|GetMaxWalkSpeed (Variables|Character|GetCharacterMovement)) (Variables|MechOptions|GetMechMaxSpeed))) 2.0) "CameraLocal" "0, 0, 0")
    (Development|PrintString "+++HitEvent+++" false)))

(event EventOnLanded
  (params (Hit :type Hit%20Result%20Structure%20%28by%20ref%29))
  (bind _debuganimbasepos (Variables|MechInfos|GetDebugAnimBasePos))
  (bind (_location _rotation) (Math|Transform|BreakTransform _debuganimbasepos))
  (bind (_x _y _z) (Class|KismetMathLibrary|BreakVector3f _location))
  (bind (_roll _pitch _yaw) (Math|Rotator|BreakRotator _rotation))
  (Development|PrintString "Landed")
  (Variables|/Script/Engine.CharacterMovementComponent|SetMaxWalkSpeed (Variables|Character|GetCharacterMovement) 0.0)
  (CameraShakes|StartCameraShake (Variables|/Script/Engine.PlayerController|GetPlayerCameraManager (Variables|References|GetPlayerController)) "/Game/Effects/CS_WallCrash.CS_WallCrash_C" 1.0 "CameraLocal" "0, 0, 0")
  (Utilities|FlowControl|Delay 1.0)
  (Variables|/Script/Engine.CharacterMovementComponent|SetMaxWalkSpeed (Variables|Character|GetCharacterMovement) (* (Variables|MechInfos|GetCurrentMechEnginePower) (Variables|MechOptions|GetMechMaxSpeed)))
  ;[1 1 0] Starting placeholder Timeline Animation for Cockpit swaying
  (bind (_direction _xbobbing _ybobbing _zbobbing _pitchswaying _rollswaying) (Timeline|DebugMechMovement Play)
    (:Update
      (Transformation|SetRelativeTransform (Variables|Default|GetCockpitBase) (Math|Transform|MakeTransform (Math|Vector|MakeVector (+ (* _xbobbing 0.2) _x) (+ (* _ybobbing 3e+01) _y) (+ (* _zbobbing 4e+01) _z)) (Math|Rotator|MakeRotator (+ (* _rollswaying 0.5) _roll) (+ (* _pitchswaying 1.0) _pitch) _yaw)) false false)
      (Components|Timeline|SetPlayRate (Variables|Default|GetDebugMechMovement) (/ (/ (Variables|MechInfos|GetHorizontalVelocity) (Variables|/Script/Engine.CharacterMovementComponent|GetMaxWalkSpeed (Variables|Character|GetCharacterMovement))) 1.7)))
    (:EventTrack
      (CallFunction|OnStep))))

(event EventOnWalkingOffLedge
  (params (PreviousFloorImpactNormal :type Vector%20%28by%20ref%29 :default "0, 0, 0") (PreviousFloorContactNormal :type Vector%20%28by%20ref%29 :default "0, 0, 0") (PreviousLocation :type Vector%20%28by%20ref%29 :default "0, 0, 0") (TimeDelta :type Float%20%28single-precision%29))
  (bind _debuganimbasepos (Variables|MechInfos|GetDebugAnimBasePos))
  (bind (_location _rotation) (Math|Transform|BreakTransform _debuganimbasepos))
  (bind (_x _y _z) (Class|KismetMathLibrary|BreakVector3f _location))
  (bind (_roll _pitch _yaw) (Math|Rotator|BreakRotator _rotation))
  (Development|PrintString "Started falling")
  ;[1 1 0] Starting placeholder Timeline Animation for Cockpit swaying
  (bind (_direction _xbobbing _ybobbing _zbobbing _pitchswaying _rollswaying) (Timeline|DebugMechMovement Stop)
    (:Update
      (Transformation|SetRelativeTransform (Variables|Default|GetCockpitBase) (Math|Transform|MakeTransform (Math|Vector|MakeVector (+ (* _xbobbing 0.2) _x) (+ (* _ybobbing 3e+01) _y) (+ (* _zbobbing 4e+01) _z)) (Math|Rotator|MakeRotator (+ (* _rollswaying 0.5) _roll) (+ (* _pitchswaying 1.0) _pitch) _yaw)) false false)
      (Components|Timeline|SetPlayRate (Variables|Default|GetDebugMechMovement) (/ (/ (Variables|MechInfos|GetHorizontalVelocity) (Variables|/Script/Engine.CharacterMovementComponent|GetMaxWalkSpeed (Variables|Character|GetCharacterMovement))) 1.7)))
    (:EventTrack
      (CallFunction|OnStep))))

(event Custom|CustomEvent
  ;[1 0 0] Damage Events
  (Niagara|SpawnSystematLocation "/Game/Effects/ParticleEffects/NS_PomPomImpact.NS_PomPomImpact" (Transformation|GetActorLocation))
  (Actor|DestroyActor))

(event Custom|CustomEvent_1
  ;[1 0 0] Damage Events
  (Development|PrintString "Mech health below 25%"))

(event Custom|CustomEvent_2
  ;[1 0 0] Damage Events
  (Development|PrintString "Mech health below 50%"))

(event Custom|CustomEvent_3
  ;[1 0 0] Damage Events
  (Development|PrintString "Mech health below 75%"))

(event Custom|CustomEvent_4
  (params (DamageTaken :type Integer) (Instigator :type Actor%20Object%20Reference) (HitLocation :type Vector))
  (bind (_x _y) (Class|KismetMathLibrary|BreakVector3f HitLocation))
  (bind _returnvalue (Transformation|GetActorLocation))
  (bind _returnvalue_2 (Math|Vector|MakeVector _x _y 0.0))
  (bind (_x_2 _y_2) (Class|KismetMathLibrary|BreakVector3f _returnvalue))
  (bind _returnvalue_3 (Math|Vector|MakeVector _x_2 _y_2 0.0))
  (bind _returnvalue_4 (- _returnvalue_3 _returnvalue_2))
  (bind _returnvalue_5 (Math|Vector|Normalize _returnvalue_4))
  ;[1 0 0] Damage Events
  (Default|CallMechTookDamage)
  (Camera|PlayWorldCameraShake "/Game/Effects/CS_MinorHit.CS_MinorHit_C" HitLocation 0.0 5e+02)
  (Development|PrintString "Mech took damage")
  (Development|PrintString (Utilities|String|ToString(Vector) _returnvalue_5))
  (Variables|/Script/Engine.MovementComponent|SetVelocity (Variables|Character|GetCharacterMovement) (+ (Variables|/Script/Engine.MovementComponent|GetVelocity (Variables|Character|GetCharacterMovement)) (* _returnvalue_5 64.0))))

(fn ConstructionScript)

(fn SetMechState
  (params (NewMechState :type E_MechStates%20Enum :default "NewEnumerator0"))
  (LocalVariables|Setvalue NewMechState)
  (Utilities|FlowControl|Sequence
    (:then_0
      ;[1 1 1] Check for special situations
      (switch Utilities|FlowControl|Switch|SwitchonE_MechStates (Variables|MechInfos|GetCurrentState)
        (:NewEnumerator0
          (switch Utilities|FlowControl|Switch|SwitchonE_MechStates (LocalVariables|Getvalue)
            (:NewEnumerator1
              (Development|PrintString "Started the Mech")
              (CallFunction|OnMechStart))))))
    (:then_1
      ;[1 1 1] Set value
      (Variables|MechInfos|SetCurrentState (LocalVariables|Getvalue)))))

(fn SetControlled
  (params (value :type Boolean))
  (bind _output_get (Variables|MechInfos|SetControlled value))
  (if _output_get
    _
    (else
      _))
  (return _output_get))

(fn Steering
  (bind _placholdersteerstickrot (Variables|MechInfos|GetPlacholderSteerStickRot))
  (bind (_roll _pitch) (Math|Rotator|BreakRotator _placholdersteerstickrot))
  (Utilities|FlowControl|Sequence
    (:then_0
      (Utilities|FlowControl|Sequence
        (:then_0
          ;[1 1 1] Method 2: Clamping Input to 1. Forces a constant movement with the mouse and puts a ceiling on "stick speed"
          (if (Variables|MechInfos|GetControlled)
            (Variables|MechInfos|SetMechSteerIs (Class|KismetMathLibrary|ClampAxes2D (+ (Variables|MechInfos|GetMechSteerIs) (* (Variables|/Game/Blueprints/PC_PlayerController.PC_PlayerController_C|GetSteerInput (Variables|References|GetPlayerController)) (Variables|Default|GetDeltaTime))) -1.0 1.0))))
        (:then_1
          ;[1 1 0] Move Steerstick
          (Transformation|SetRelativeRotation (Variables|Default|GetSteerStick) (Math|Rotator|MakeRotator (+ (.X (Math|Vector2D|BreakVector2D (* (Variables|MechInfos|GetMechSteerIs) "(X=20.000000,Y=-20.000000)"))) _roll) (+ (.Y (Math|Vector2D|BreakVector2D (* (Variables|MechInfos|GetMechSteerIs) "(X=20.000000,Y=-20.000000)"))) _pitch) 0.0) false false))))
    (:then_1
      (switch Utilities|FlowControl|Switch|SwitchonE_MechStates (Variables|MechInfos|GetCurrentState)
        (:NewEnumerator1
          (Utilities|FlowControl|Sequence
            (:then_0
              ;[1 1 1] Turn
              (Transformation|AddActorLocalRotation self (Math|Rotator|MakeRotator 0.0 0.0 (* (* (.X (Math|Vector2D|BreakVector2D (Variables|MechInfos|GetMechSteerIs))) (Variables|Default|GetDeltaTime)) (Variables|MechOptions|GetMaxTurnSpeed))) false false))
            (:then_1
              ;[1 1 1] Move
              (bind _output_get (Variables|MechInfos|SetCurrentMechEnginePower (Math|Float|SelectFloat 0.0 (Math|Float|Lerp (Variables|MechInfos|GetCurrentMechEnginePower) (/ (+ (.Y (Math|Vector2D|BreakVector2D (Variables|MechInfos|GetMechSteerIs))) 1.0) 2.0) (* (Variables|Default|GetDeltaTime) 0.5)) (Math|Float|NearlyEqual(Float) (Math|Float|Lerp (Variables|MechInfos|GetCurrentMechEnginePower) (/ (+ (.Y (Math|Vector2D|BreakVector2D (Variables|MechInfos|GetMechSteerIs))) 1.0) 2.0) (* (Variables|Default|GetDeltaTime) 0.5)) 0.0 0.005))))
              (Development|PrintString (Utilities|String|Append (Utilities|String|MakeLiteralString "EnginePower: ") (Utilities|String|ToString(Float) _output_get)) true false "(R=0.000000,G=0.660000,B=1.000000,A=1.000000)" 0.0)
              (Variables|/Script/Engine.CharacterMovementComponent|SetMaxWalkSpeed (Variables|Character|GetCharacterMovement) (* (Variables|MechInfos|GetCurrentMechEnginePower) (Variables|MechOptions|GetMechMaxSpeed)))
              (Pawn|Input|AddMovementInput (Transformation|GetActorForwardVector) (Math|Float|Sign(Float) (Variables|MechInfos|GetCurrentMechEnginePower)) false)
              (Development|PrintString (Utilities|String|Append (Utilities|String|MakeLiteralString "WalkSpeed: ") (Utilities|String|ToString(Float) (Math|Vector|VectorLengthXY (Pawn|Components|CharacterMovement|GetLastUpdateVelocity (Variables|Character|GetCharacterMovement))))) true false "(R=0.000000,G=0.660000,B=1.000000,A=1.000000)" 0.0))))))))

(fn ChangeEntityHP
  (params (HP%20Change%20Mode :type E_HPChangeType%20Enum :default "NewEnumerator1") (Value :type Integer) (HitLocation :type Vector :default "0, 0, 0") (Instigator :type Actor%20Object%20Reference))
  (bind _isded (Default|ChangeHP (Variables|Default|GetHit%20Point%20System) HP%20Change%20Mode Value HitLocation Instigator))
  (return true _isded))

(fn GetCharacterMovementComponent
  (return (Variables|Character|GetCharacterMovement)))

(fn GetGroundWorldPosition
  (bind _returnvalue (Transformation|GetActorLocation))
  (bind (_x _y _z) (Math|Vector|BreakVector _returnvalue))
  (return (Math|Vector|MakeVector _x _y (- _z (Components|Capsule|GetScaledCapsuleHalfHeight (Variables|Collision|GetCapsuleComponent))))))

(fn GetHealthComponent
  (return (Variables|Default|GetHit%20Point%20System)))