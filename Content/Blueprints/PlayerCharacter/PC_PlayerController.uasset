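; Player controller that links the Johanna pawn and Brass Bull mech at BeginPlay and routes Enhanced Input for them.
; Directional input becomes steering unless the camera is unlocked; interact presses fire start/stop dispatchers.
; Debug inputs move Johanna into the mech, start or damage it, switch enemy AI state and emit noise.
; A time-weighted input smoothing function reads a prefilled sample buffer, but the code updating that buffer is disconnected.
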(event Input|EnhancedActionEvents|EnhancedInputActionIA_Interact
  (params (ActionValue :type Boolean) (ElapsedSeconds :type Float%20%28double-precision%29) (TriggeredSeconds :type Float%20%28double-precision%29) (InputAction :type Input%20Action%20Object%20Reference :default "/Game/Input/IA_Interact.IA_Interact"))
  (:Started
    (Default|CallInteractionButtonStart))
  (:Completed
    (Default|CallInteractionButtonStop)))

(event Input|EnhancedActionEvents|EnhancedInputActionIA_UnlockView
  (params (ActionValue :type Boolean) (ElapsedSeconds :type Float%20%28double-precision%29) (TriggeredSeconds :type Float%20%28double-precision%29) (InputAction :type Input%20Action%20Object%20Reference :default "/Game/Input/IA_UnlockView.IA_UnlockView"))
  (:Started
    (Variables|PlayerControllerInfos|SetCameraUnlocked ActionValue :!label _label))
  (:Completed
    (goto _label)))

(event Input|EnhancedActionEvents|EnhancedInputActionIA_Directional
  (params (ActionValue :type Vector%202D%20Structure) (ElapsedSeconds :type Float%20%28double-precision%29) (TriggeredSeconds :type Float%20%28double-precision%29) (InputAction :type Input%20Action%20Object%20Reference :default "/Game/Input/IA_Directional.IA_Directional"))
  (:Triggered
    (bind _output_get (Variables|PlayerControllerInfos|SetDirectionalInput ActionValue))
    (if (Variables|PlayerControllerInfos|GetCameraUnlocked)
      (Variables|PlayerControllerInfos|SetSteerInput "" :!label _label)
      (else
        (Variables|PlayerControllerInfos|SetSteerInput _output_get))))
  (:Completed
    (Variables|PlayerControllerInfos|SetDirectionalInput "")
    (goto _label)))

(event Input|EnhancedActionEvents|EnhancedInputActionIA_DebugStart
  (params (ActionValue :type Boolean) (ElapsedSeconds :type Float%20%28double-precision%29) (TriggeredSeconds :type Float%20%28double-precision%29) (InputAction :type Input%20Action%20Object%20Reference :default "/Game/Input/IA_DebugStart.IA_DebugStart"))
  (bind _johanna (Variables|References|GetJohanna))
  (:Started
    (switch Utilities|FlowControl|Switch|SwitchonE_JohannaStates (Variables|/Game/Blueprints/PlayerCharacter/PWN_Johanna.PWN_Johanna_C|GetCurrentOccupation (Variables|References|GetJohanna))
      (:NewEnumerator0
        ;[1 1 0] Placeholder Start into Mech
        (Variables|/Game/Blueprints/PlayerCharacter/PWN_Johanna.PWN_Johanna_C|SetCurrentOccupation (Variables|References|GetJohanna) "NewEnumerator1")
        (bind _asbp_johanna_slot (Utilities|Casting|CastToBP_JohannaSlot (Variables|/Script/Engine.ChildActorComponent|GetChildActor (Variables|/Game/Blueprints/PlayerCharacter/CHR_Mech.CHR_Mech_C|GetBP_JohannaSlot (Variables|References|GetBrassBull))))
          (:then
            (Variables|/Game/Blueprints/PlayerCharacter/PWN_Johanna.PWN_Johanna_C|SetMoveTarget (Variables|References|GetJohanna) _asbp_johanna_slot)
            (Variables|/Game/Blueprints/PlayerCharacter/PWN_Johanna.PWN_Johanna_C|SetTransitionStartPos _johanna (Transformation|GetActorTransform _johanna)))
          (:CastFailed
            (Development|PrintString "Wait, what?"))))
      (:NewEnumerator2
        (Default|StartMech (Variables|References|GetBrassBull))))))

(event EventBeginPlay
  (Development|PrintString "PlayerController online")
  (Utilities|FlowControl|Sequence
    (:then_0
      (CallFunction|InitializeEnhancedInput))
    (:then_1
      ;[1 1 1] Find Johanna Pawn
      (bind _returnvalue (Actor|GetActorOfClass "/Game/Blueprints/PlayerCharacter/PWN_Johanna.PWN_Johanna_C"))
      (Utilities|IsValid _returnvalue
        (:Is%20Valid
          (Variables|References|SetJohanna _returnvalue)
          (Development|PrintString "Johanna found."))
        (:Is%20Not%20Valid
          (Development|PrintString "Couldn't find Johanna pawn."))))
    (:then_2
      ;[1 1 1] Find Brass Bull Mech
      (bind _returnvalue_2 (Actor|GetActorOfClass "/Game/Blueprints/PlayerCharacter/CHR_Mech.CHR_Mech_C"))
      (Utilities|IsValid _returnvalue_2
        (:Is%20Valid
          (Variables|References|SetBrassBull _returnvalue_2)
          (Development|PrintString "Brass Bull found."))
        (:Is%20Not%20Valid
          (Development|PrintString "Couldn't find Brass Bull."))))
    (:then_3
      (Variables|/Game/Blueprints/PlayerCharacter/PWN_Johanna.PWN_Johanna_C|SetPlayerController (Variables|References|GetJohanna) self)
      (Variables|/Game/Blueprints/PlayerCharacter/PWN_Johanna.PWN_Johanna_C|SetBrassBull (Variables|References|GetJohanna) (Variables|References|GetBrassBull))
      (Default|EventonControllerConnection (Variables|References|GetJohanna))
      (Actor|Tick|SetActorTickEnabled (Variables|References|GetJohanna) true)
      (bind _output_get (Variables|/Game/Blueprints/PlayerCharacter/CHR_Mech.CHR_Mech_C|SetPlayerController (Variables|References|GetBrassBull) self))
      (Actor|Tick|SetActorTickEnabled _output_get true)
      (Variables|/Game/Blueprints/PlayerCharacter/CHR_Mech.CHR_Mech_C|SetJohanna (Variables|References|GetBrassBull) (Variables|References|GetJohanna)))))

(event EventTick
  (params (DeltaSeconds :type Float%20%28single-precision%29))
  (Variables|Default|SetDeltaTime DeltaSeconds))

(event Input|KeyboardEvents|DebugKey5
  (params (Key :type Key%20Structure :default "None") (ActionValue :type Input%20Action%20Value%20Structure))
  (bind _self self)
  (bind _returnvalue (Pawn|GetControlledPawn _self))
  (bind _returnvalue_2 (Transformation|GetActorLocation _returnvalue))
  ;[1 1 0] AI Test actions
  (:Pressed
    (Development|PrintString "Johanna makes noise")
    (Class|Actor|MakeNoise 1.0 _returnvalue _returnvalue_2 0.0 "None")
    (Audio|PlaySoundatLocation "/Engine/VREditor/Sounds/VR_teleport.VR_teleport" _returnvalue_2 "0, 0, 0" 1.0 1.0 0.0 0 0 0 0)))

(event Input|KeyboardEvents|DebugKey2
  (params (Key :type Key%20Structure :default "None") (ActionValue :type Input%20Action%20Value%20Structure))
  ;[1 1 0] AI Test actions
  (:Pressed
    (Development|PrintString "AttackBB")
    (bind _returnvalue (Actor|GetActorOfClass "/Game/Blueprints/Enemies/EnemyBase/BP_Enemy_Base.BP_Enemy_Base_C"))
    (bind _asaic_enemy_base (Utilities|Casting|CastToAIC_Enemy_Base (AI|GetAIController _returnvalue)))
    (Default|SetStateasinCombat _asaic_enemy_base (Variables|References|GetBrassBull))))

(event Input|KeyboardEvents|DebugKey1
  (params (Key :type Key%20Structure :default "None") (ActionValue :type Input%20Action%20Value%20Structure))
  ;[1 1 0] AI Test actions
  (:Pressed
    (Development|PrintString "Idle")
    (bind _returnvalue (Actor|GetActorOfClass "/Game/Blueprints/Enemies/EnemyBase/BP_Enemy_Base.BP_Enemy_Base_C"))
    (bind _asaic_enemy_base (Utilities|Casting|CastToAIC_Enemy_Base (AI|GetAIController _returnvalue)))
    (Default|SetStateasPassive _asaic_enemy_base)))

(event Input|KeyboardEvents|DebugKeyK
  (params (Key :type Key%20Structure :default "None") (ActionValue :type Input%20Action%20Value%20Structure))
  ;[1 1 0] Debug kill switch
  (:Pressed
    (Default|ChangeHP (Variables|/Game/Blueprints/PlayerCharacter/CHR_Mech.CHR_Mech_C|GetHit%20Point%20System (Variables|References|GetBrassBull)) "NewEnumerator1" -500 "0, 0, 0")))

(fn ConstructionScript
  (for _index (range 1 180)
    (Utilities|Array|Add (Variables|PlayerControllerInfos|GetInputSampleArray) (Utilities|Struct|MakeF_InputSample_Vector2 "(X=0.000000,Y=0.000000)" 0.01667))))

(fn InitializeEnhancedInput
  (bind _aspc_player_controller (Utilities|Casting|CastToPC_PlayerController (Game|GetPlayerController 0))
    (:then
      (Input|AddMappingContext (PlayerController|LocalPlayerSubsystems|GetEnhancedInputLocalPlayerSubsystem _aspc_player_controller) "/Game/Input/Default.Default" 0 "(bIgnoreAllPressedKeysUntilRelease=True,bForceImmediately=False)")
      (Development|PrintString "Enhanced Input initialized"))
    (:CastFailed
      (Development|PrintString "PlayerIndex0 has wrong PlayerController"))))

(fn GetSmoothedInput
  (params (Smoothing%20Time :type Float%20%28double-precision%29))
  (bind _inputsamplearray (Variables|PlayerControllerInfos|GetInputSampleArray))
  (LocalVariables|SetSmoothingTime Smoothing%20Time)
  (bind _array_index (Utilities|Array|ForEachLoopwithBreak (Variables|PlayerControllerInfos|GetInputSampleArray) :!label _label)
    (:LoopBody
      ;[1 1 1] Add InputSample to the pile.
      (LocalVariables|SetCulmativeInput (+ (LocalVariables|GetCulmativeInput) (* (.FrameInput (Utilities|Struct|BreakF_InputSample_Vector2 (Utilities|Array|Get(acopy) _inputsamplearray (- (Utilities|Array|Length _inputsamplearray) (+ _array_index 1))))) (/ (- (LocalVariables|GetSmoothingTime) (LocalVariables|GetCulmativeSampleTime)) (LocalVariables|GetSmoothingTime)))))
      (Math|Integer|IncrementInt (LocalVariables|GetEvaluatedSamples)
        (:%20%20
          (if (>= (LocalVariables|GetCulmativeSampleTime) (LocalVariables|GetSmoothingTime))
            (goto _label Break)
            (else
              (LocalVariables|SetCulmativeSampleTime (+ (LocalVariables|GetCulmativeSampleTime) (.FrameTime (Utilities|Struct|BreakF_InputSample_Vector2 (Utilities|Array|Get(acopy) _inputsamplearray (- (Utilities|Array|Length _inputsamplearray) (+ _array_index 1))))))))))))
    (:Completed
      ;[1 1 1] Output final smoothed input value
      (return (/ (LocalVariables|GetCulmativeInput) (Math|Conversions|ToFloat(Integer) (LocalVariables|GetEvaluatedSamples)))))))

(fn VehicleTookDamage)